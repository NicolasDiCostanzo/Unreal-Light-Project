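; BP_spot is a spotlight Blueprint that tints its SpotLight component according to a ColorEnum value.
; On BeginPlay, SetColorFromEnum maps the enum to one of seven preset colors, stores it in SpotColor and applies it as the light color.
; The Red case only stores SpotColor and never reaches the SetLightColor call, so the light keeps its existing color.
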(event EventBeginPlay
  (CallFunction|SetColorfromEnum))

(fn ConstructionScript)

(fn SetColorfromEnum
  (switch Utilities|FlowControl|Switch|SwitchonColor_enum (Variables|Default|GetColor_enum)
    (:NewEnumerator0
      (Variables|Default|SetspotColor "(R=1.000000,G=1.000000,B=0.000000,A=1.000000)")
      (Rendering|Components|Light|SetLightColor (Variables|Default|GetSpotLight) (Variables|Default|GetspotColor) true :!label _label))
    (:NewEnumerator1
      (Variables|Default|SetspotColor "(R=1.000000,G=1.000000,B=1.000000,A=1.000000)")
      (goto _label))
    (:NewEnumerator2
      (Variables|Default|SetspotColor "(R=0.000000,G=0.000000,B=0.000000,A=1.000000)")
      (goto _label))
    (:NewEnumerator3
      (Variables|Default|SetspotColor "(R=0.000000,G=1.000000,B=0.000000,A=1.000000)")
      (goto _label))
    (:NewEnumerator4
      (Variables|Default|SetspotColor "(R=1.000000,G=0.000000,B=0.000000,A=1.000000)"))
    (:NewEnumerator5
      (Variables|Default|SetspotColor "(R=1.000000,G=0.500000,B=0.000000,A=1.000000)")
      (goto _label))
    (:NewEnumerator6
      (Variables|Default|SetspotColor "(R=0.000000,G=0.000000,B=1.000000,A=1.000000)")
      (goto _label))))