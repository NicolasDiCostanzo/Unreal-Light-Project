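; Activable platform Blueprint that moves its Cube when switched on and returns it when switched off.
; CallActiver and CallDesactiver set the EstActive flag and play or reverse a single timeline.
; Each timeline update feeds its Activer track to BougerPlateforme, which converts that alpha through an Activer call into the Cube's relative location, without sweep.
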(event EventCallDesactiver
  (Variables|Default|SetestActive false)
  (bind _activer (Timeline|Timeline_1 Reverse)
    (:Update
      (CallFunction|BougerPlateforme _activer))))

(event EventCallActiver
  (Variables|Default|SetestActive true)
  (bind _activer (Timeline|Timeline_1 Play)
    (:Update
      (CallFunction|BougerPlateforme _activer))))

(event EventBeginPlay)

(fn ConstructionScript
  (|CallParentFunction))

(fn BougerPlateforme
  (params (Alpha :type Float%20%28single-precision%29))
  (bind _nouvelleposition (CallFunction|Activer Alpha))
  (Transformation|SetRelativeLocation (Variables|Default|GetCube) _nouvelleposition false false))