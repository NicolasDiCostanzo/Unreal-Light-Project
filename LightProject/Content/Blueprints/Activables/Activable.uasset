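; Activable is an object that switches on and off according to how many lights it currently has.
; AjouterLumiere and EnleverLumiere adjust the light counter, setting EstActive through CallActiver when it reaches the required total and through CallDesactiver when it falls below.
; Activer only returns a position interpolated between Depart and Arrivee by an Alpha; nothing here calls it or moves anything.
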(fn ConstructionScript)

(fn EnleverLumiere
  (bind _result (Math|Integer|DecrementInt (Variables|Default|GetnbrLumieresActuelles))
    (:%20%20
      (if (< _result (Variables|Default|GetnbrTotalLumieres))
        (CallFunction|CallDesactiver)
        (Development|PrintString "call desactiver")
        (else
          (Development|PrintString "pas <"))))))

(fn AjouterLumiere
  (bind _result (Math|Integer|IncrementInt (Variables|Default|GetnbrLumieresActuelles))
    (:%20%20
      (if (>= _result (Variables|Default|GetnbrTotalLumieres))
        (CallFunction|CallActiver)))))

(fn Activer
  (params (Alpha :type Float%20%28single-precision%29))
  (return (Math|Vector|Lerp(Vector) (Variables|/Script/Engine.SceneComponent|GetRelativeLocation (Variables|Default|GetDepart)) (Variables|/Script/Engine.SceneComponent|GetRelativeLocation (Variables|Default|GetArrivee)) Alpha)))

(fn CallActiver
  (Variables|Default|SetestActive true)
  (Development|PrintString "call activer"))

(fn CallDesactiver
  (Variables|Default|SetestActive false))