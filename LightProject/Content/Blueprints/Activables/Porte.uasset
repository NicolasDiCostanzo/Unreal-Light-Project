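; Activable door Blueprint that slides open and closed when activated or deactivated.
; Activation sets the active flag and plays the BougerActiver timeline; deactivation clears it and reverses the same timeline.
; Each timeline update passes its alpha through BougerPorte, which uses the Activer function to compute the Porte component's relative location and sets it without sweep.
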(event EventBeginPlay
  (|CallParentFunction))

(event EventCallActiver
  (Variables|Default|SetestActive true)
  (bind _activer (Timeline|BougerActiver Play)
    (:Update
      (CallFunction|BougerPorte _activer))))

(event EventCallDesactiver
  (Variables|Default|SetestActive false)
  (bind _activer (Timeline|BougerActiver Reverse)
    (:Update
      (CallFunction|BougerPorte _activer))))

(fn ConstructionScript
  (|CallParentFunction))

(fn BougerPorte
  (params (Alpha :type Float%20%28single-precision%29))
  (bind _nouvelleposition (CallFunction|Activer Alpha))
  (Transformation|SetRelativeLocation (Variables|Components|GetPorte) _nouvelleposition false false))