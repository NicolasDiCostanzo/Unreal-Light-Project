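; BP_spot is a colored light actor that shows a text prompt, noted as a "press e" display, while the player is nearby.
; On BeginPlay, a color enum selects the color applied to both its spot light and point light.
; Trigger box overlaps with the player pawn toggle the text's visibility.
; Every tick, the text rotates from the camera rotation to face the player, billboard-style; no key input is handled here.
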(event OnComponentBeginOverlap(triggerBox)
  (params (OverlappedComponent :type Primitive%20Component%20Object%20Reference) (OtherActor :type Actor%20Object%20Reference) (OtherComp :type Primitive%20Component%20Object%20Reference) (OtherBodyIndex :type Integer) (bFromSweep :type Boolean) (SweepResult :type Hit%20Result%20Structure%20%28by%20ref%29))
  ;[1 1 1] press e display
  (if (== OtherActor (Game|Player|GetPlayerPawn 0))
    (Rendering|SetVisibility (Variables|Default|GetTextRender) true false)))

(event OnComponentEndOverlap(triggerBox)
  (params (OverlappedComponent :type Primitive%20Component%20Object%20Reference) (OtherActor :type Actor%20Object%20Reference) (OtherComp :type Primitive%20Component%20Object%20Reference) (OtherBodyIndex :type Integer))
  ;[1 1 1] press e display
  (if (== OtherActor (Game|Player|GetPlayerPawn 0))
    (Rendering|SetVisibility (Variables|Default|GetTextRender) false false)))

(event EventBeginPlay
  (CallFunction|SetColorfromEnum))

(event EventTick
  (params (DeltaSeconds :type Float%20%28single-precision%29))
  (CallFunction|SetTextRotation))

(fn ConstructionScript)

(fn SetColorfromEnum
  (switch Utilities|FlowControl|Switch|SwitchonColor_enum (Variables|Default|GetColor_enum)
    (:NewEnumerator0
      (Variables|Default|SetspotColor "(R=1.000000,G=1.000000,B=0.000000,A=1.000000)"))
    (:NewEnumerator1
      (Variables|Default|SetspotColor "(R=0.215861,G=0.000000,B=0.215861,A=1.000000)"))
    (:NewEnumerator2
      (Variables|Default|SetspotColor "(R=1.000000,G=0.078431,B=0.576471,A=1.000000)"))
    (:NewEnumerator3
      (Variables|Default|SetspotColor "(R=0.000000,G=1.000000,B=0.000000,A=1.000000)"))
    (:NewEnumerator4
      (Variables|Default|SetspotColor "(R=1.000000,G=0.000000,B=0.000000,A=1.000000)"))
    (:NewEnumerator5
      (Variables|Default|SetspotColor "(R=0.744792,G=0.242191,B=0.000000,A=1.000000)"))
    (:NewEnumerator6
      (Variables|Default|SetspotColor "(R=0.000000,G=0.000000,B=1.000000,A=1.000000)")))
  (Rendering|Components|Light|SetLightColor (Variables|Default|GetSpotLight) (Variables|Default|GetspotColor) true)
  (Rendering|Components|Light|SetLightColor (Variables|Default|GetPointLight) (Variables|Default|GetspotColor) true))

(fn SetTextRotation
  (bind _returnvalue (Game|GetPlayerCameraManager 0))
  (bind _returnvalue_2 (Camera|GetCameraRotation _returnvalue))
  (Transformation|SetWorldRotation (Variables|Default|GetTextRender) (Math|Rotator|MakeRotator (+ (.roll _returnvalue_2) 1.8e+02) (+ (.pitch _returnvalue_2) 1.8e+02) (.yaw _returnvalue_2)) false false))